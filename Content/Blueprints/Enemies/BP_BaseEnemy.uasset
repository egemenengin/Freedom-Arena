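; Base enemy Blueprint that handles health bar and floating hit-number UI on top of its parent class.
; BeginPlay links the health bar widget component to this enemy, and show/hide events toggle its visibility, with show also calling the parent implementation.
; Each hit spawns an animated WBP_Hit with damage amount and headshot flag, projected to screen and registered with its world location via AddHitWidget.
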(event `self.ReceiveBeginPlay`
  (bind _aswbp_enemy_health_bar (cast `/Game/Blueprints/HUD/WBP_EnemyHealthBar` (`WidgetComponent.GetUserWidgetObject` (`self.HealthBarWidget`))))
  (set `/Game/Blueprints/HUD/WBP_EnemyHealthBar.Enemy` self _aswbp_enemy_health_bar))

(event `self.ShowHealthBar`
  ;[1 0.2292 0.2292] HealthBar Handle
  (`Widget.SetVisibility` (`WidgetComponent.GetUserWidgetObject` (`self.HealthBarWidget`)) "Visible")
  (`parent.ShowHealthBar`))

(event `self.HideHealthBar`
  ;[1 0.2292 0.2292] HealthBar Handle
  (`Widget.SetVisibility` (`WidgetComponent.GetUserWidgetObject` (`self.HealthBarWidget`)) "Hidden"))

(event `self.ShowHitAmount`
  (params (HitAmount :type "Float (single-precision)") (HitLocation :type "Vector Structure") (isHeadShot :type Boolean))
  (bind _returnvalue (`|CreateWidget` "/Game/Blueprints/HUD/WBP_Hit.WBP_Hit_C"))
  (`UserWidget.AddToViewport` _returnvalue 0)
  (set `/Game/Blueprints/HUD/WBP_Hit.HitAmount` (`KismetTextLibrary.Conv_DoubleToText` HitAmount "HalfToEven") _returnvalue)
  (`self.AddHitWidget` _returnvalue HitLocation)
  (`UserWidget.SetPositionInViewport` _returnvalue (`GameplayStatics.ProjectWorldToScreen` (`GameplayStatics.GetPlayerController` 0) HitLocation) true)
  (set `/Game/Blueprints/HUD/WBP_Hit.bIsHeadShot` isHeadShot _returnvalue)
  (`UserWidget.PlayAnimation` _returnvalue (`/Game/Blueprints/HUD/WBP_Hit.HitTextAnimation` _returnvalue) 0.0 1 "Forward" 1.0 false))

(fn `UserConstructionScript`)